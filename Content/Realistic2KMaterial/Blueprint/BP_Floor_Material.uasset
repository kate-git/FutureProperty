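; Construction-script actor for a configurable floor piece that assigns a chosen static mesh and per-section materials.
; UVset creates dynamic material instances per slot and pushes color, UV, roughness, material and displacement parameters from arrays resized to the material count.
; Optional centimeter sizing scales X and Y from the mesh bounding box, and an optional fix multiplies UV scale by that factor to keep tiling consistent.
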(fn `GetStaticSize`
  (params (Target :type "StaticMesh Object Reference"))
  (returns (X :type "Float (double-precision)") (Y :type "Float (double-precision)") (Z :type "Float (double-precision)"))
  (bind (_min _max) (break `Box` (`StaticMesh.GetBoundingBox` Target)))
  (return (.x (- _max _min)) (.y (- _max _min)) (.z (- _max _min))))

(fn `SetstaticMeshAndMaterialArray`
  (params (Target :type "StaticMeshComponent Object Reference") (NewMesh :type "StaticMesh Object Reference") (Array :type "Array of MaterialInstance Object Reference"))
  (`StaticMeshComponent.SetStaticMesh` Target NewMesh)
  (`KismetArrayLibrary.Array_Resize` Array (`StaticMesh.GetNumSections` NewMesh 0))
  (for _index (range (`PrimitiveComponent.GetNumMaterials` Target))
    (`PrimitiveComponent.SetMaterial` Target _index (`|GetArrayItem` Array _index))))

(fn `UserConstructionScript`
  (`self.SetstaticMeshAndMaterialArray` (`self.SM_MaterialFloor`) (`self.New Mesh`) (`self.Material`))
  (`self.UVset` (`self.SM_MaterialFloor`) (`self.New Mesh`) (`self.Material`) (`self.UVSCale`) (`self.UVSOffset`) (`self.UVRotation Degree`) (`self.UVMaterialoffset`) (`self.UVRoughnessoffset`) (`self.Color Multiply`) (`self.Color Add`) true (`self.UvDisplacementmultiply`) (`self.Displacement Add`)))

(fn `UVset`
  (params (Target :type "PrimitiveComponent Object Reference") (Target1 :type "StaticMesh Object Reference") (`MI Array` :type "Array of MaterialInstance Object Reference (by ref)") (UVSCale :type "Array of Vector Structure (by ref)") (UVSOffset :type "Array of Vector Structure (by ref)") (UVRotationDegree :type "Array of Float (double-precision) (by ref)") (UVMaterialoffset :type "Array of Float (double-precision) (by ref)") (UVRoughnessoffset :type "Array of Float (double-precision) (by ref)") (ColorMultiply :type "Array of LinearColor Structure (by ref)") (ColorAdd :type "Array of LinearColor Structure") (DoScale :type Boolean) (DisplacementMultiply :type "Array of Float (double-precision)") (DisplacementAdd :type "Array of Float (double-precision)"))
  (locals (MaterialLength :type Integer :default 0))
  (bind _returnvalue (`KismetArrayLibrary.Array_Length` `MI Array`))
  (bind (_x _y) (`self.GetStaticSize` Target1))
  (set `local.MaterialLength` _returnvalue)
  (`|ExecutionSequence`
    (:`then_0`
      (`KismetArrayLibrary.Array_Resize` UVSCale (`local.MaterialLength`))
      (`KismetArrayLibrary.Array_Resize` UVSOffset (`local.MaterialLength`))
      (`KismetArrayLibrary.Array_Resize` UVRotationDegree (`local.MaterialLength`))
      (`KismetArrayLibrary.Array_Resize` UVMaterialoffset (`local.MaterialLength`))
      (`KismetArrayLibrary.Array_Resize` UVRoughnessoffset (`local.MaterialLength`))
      (`KismetArrayLibrary.Array_Resize` ColorMultiply (`local.MaterialLength`))
      (`KismetArrayLibrary.Array_Resize` ColorAdd (`local.MaterialLength`))
      (`KismetArrayLibrary.Array_Resize` DisplacementMultiply (`local.MaterialLength`))
      (`KismetArrayLibrary.Array_Resize` DisplacementAdd (`local.MaterialLength`)))
    (:`then_1`
      ;[1 1 1] SetDeskColumnUVset
      (for _index (range _returnvalue)
        (bind _returnvalue_2 (`PrimitiveComponent.CreateDynamicMaterialInstance` Target _index null "None"))
        (`MaterialInstanceDynamic.SetVectorParameterValue` _returnvalue_2 "ColorMultiply" (`|GetArrayItem` ColorMultiply _index))
        (`MaterialInstanceDynamic.SetVectorParameterValue` _returnvalue_2 "ColorAdd" (`|GetArrayItem` ColorAdd _index))
        (`MaterialInstanceDynamic.SetVectorParameterValue` _returnvalue_2 "UVScale" (`KismetMathLibrary.Conv_VectorToLinearColor` (`|GetArrayItem` UVSCale _index)))
        (`MaterialInstanceDynamic.SetVectorParameterValue` _returnvalue_2 "UVOffset" (`KismetMathLibrary.Conv_VectorToLinearColor` (`|GetArrayItem` UVSOffset _index)))
        (`MaterialInstanceDynamic.SetScalarParameterValue` _returnvalue_2 "UVRotationDegree" (`|GetArrayItem` UVRotationDegree _index))
        (`MaterialInstanceDynamic.SetScalarParameterValue` _returnvalue_2 "Material" (`|GetArrayItem` UVMaterialoffset _index))
        (`MaterialInstanceDynamic.SetScalarParameterValue` _returnvalue_2 "Roughness" (`|GetArrayItem` UVRoughnessoffset _index))
        (`MaterialInstanceDynamic.SetScalarParameterValue` _returnvalue_2 "DisplacementMultiply" (`|GetArrayItem` DisplacementMultiply _index))
        (`MaterialInstanceDynamic.SetScalarParameterValue` _returnvalue_2 "DisplacementAdd" (`|GetArrayItem` DisplacementAdd _index))))
    (:`then_2`
      ;[1 1 1] SetWallSize
      (if DoScale
        (if (`self.SetXY/cm?`)
          (bind _output_get (set `self.Xscale` (/ (`self.WallX/cm`) _x)))
          (bind _output_get_2 (set `self.Yscale` (/ (`self.WallY/cm`) _y)))
          (`SceneComponent.SetRelativeScale3D` Target (`KismetMathLibrary.MakeVector` _output_get _output_get_2 1.0))
          (else
            (set `self.Xscale` 1.0)
            (set `self.Yscale` 1.0)
            (set `self.WallX/cm` _x)
            (set `self.WallY/cm` _y)))))
    (:`then_3`
      ;[1 1 1] FixUVScale
      (if (`self.FixUvScaleWhenTableSizeChange?`)
        (for _index_2 (range (`KismetArrayLibrary.Array_Length` UVSCale))
          (bind _returnvalue_3 (`PrimitiveComponent.CreateDynamicMaterialInstance` Target _index_2 null "None"))
          (`MaterialInstanceDynamic.SetVectorParameterValue` _returnvalue_3 "UVScale" (`KismetMathLibrary.Conv_VectorToLinearColor` (`KismetMathLibrary.MakeVector` (* (.x (`|GetArrayItem` UVSCale _index_2)) (`self.Xscale`)) (* (.y (`|GetArrayItem` UVSCale _index_2)) (`self.Yscale`)) 1.0))))))))